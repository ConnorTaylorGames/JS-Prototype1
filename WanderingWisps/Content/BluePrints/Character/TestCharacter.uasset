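; Player character for a side-scrolling underwater game, locked to its starting X position.
; Tick tilts it to floor slopes or swim velocity and keeps the camera below the water surface.
; Timers drive bubbles, swap camera and fog by height against the water, and hide view-blocking meshes through BP_FadeComponent.
; Capsule hits run multi-trace ground checks that set jump state through controller interface messages; ToggleCharacter flips the dead state.
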(event `CheckLocation`
  (bind _x (.x (`self.StartingVector`)))
  ;[1 1 1] CheckLocation
  (if (> (.x (`self.K2_GetActorLocation`)) _x)
    (`self.K2_SetActorLocation` (`KismetMathLibrary.MakeVector` _x (.y (`self.K2_GetActorLocation`)) (.z (`self.K2_GetActorLocation`))))
    (elif (< (.x (`self.K2_GetActorLocation`)) (.x (`self.StartingVector`)))
      (`self.K2_SetActorLocation` (`KismetMathLibrary.MakeVector` _x (.y (`self.K2_GetActorLocation`)) (.z (`self.K2_GetActorLocation`)))))))

(event `ClampCamera`
  (bind (_returnvalue_x _returnvalue_y _returnvalue_z) (`KismetMathLibrary.BreakVector` (`self.K2_GetActorLocation`)))
  (bind _camera (`self.Camera`))
  (bind _camera_2 (`self.Camera`))
  (bind (_returnvalue_x_2 _returnvalue_y_2) (`KismetMathLibrary.BreakVector` (`SceneComponent.K2_GetComponentLocation` _camera)))
  (bind (_returnvalue_x_3 _returnvalue_y_3 _returnvalue_z_2) (`KismetMathLibrary.BreakVector` (`SceneComponent.K2_GetComponentLocation` _camera_2)))
  (bind (_returnvalue_x_4 _returnvalue_y_4 _returnvalue_z_3) (`KismetMathLibrary.BreakVector` (`SceneComponent.K2_GetComponentLocation` (`StaticMeshActor.StaticMeshComponent` (`self.WaterSurface`)))))
  ;[1 1 1] ClampCamera
  (if (`self.Underwater?`)
    (if (>= _returnvalue_z_2 _returnvalue_z_3)
      (`SceneComponent.K2_SetWorldLocation` _camera_2 (`KismetMathLibrary.MakeVector` _returnvalue_x_3 _returnvalue_y_3 (`KismetMathLibrary.FClamp` _returnvalue_z_2 -100000.0 _returnvalue_z_3)) false true)
      (else
        (`SceneComponent.K2_SetWorldLocation` _camera (`KismetMathLibrary.VInterpTo` (`SceneComponent.K2_GetComponentLocation` _camera) (`KismetMathLibrary.MakeVector` _returnvalue_x_2 _returnvalue_y_2 (+ _returnvalue_z (`self.CameraOffsetToPlayer`))) (`GameplayStatics.GetWorldDeltaSeconds`) 0.1) false true)))))

(event `RotateToVelocity`
  (bind (_returnvalue_x _returnvalue_y) (`KismetMathLibrary.BreakVector` (`self.GetVelocity`)))
  (bind (_returnvalue_roll _returnvalue_pitch _returnvalue_yaw) (`KismetMathLibrary.BreakRotator` (`self.K2_GetActorRotation`)))
  (bind (_returnvalue_roll_2 _returnvalue_pitch_2) (`KismetMathLibrary.BreakRotator` (`KismetMathLibrary.MakeRotFromX` (`self.GetVelocity`))))
  ;[1 1 1] Rotate to movement when swimming
  (if (!= _returnvalue_y 0.0)
    (if (`NavMovementComponent.IsFalling` (`self.CharacterMovement`))
      (`self.K2_SetActorRotation` (`KismetMathLibrary.RLerp` (`self.K2_GetActorRotation`) (`KismetMathLibrary.MakeRotator` _returnvalue_roll_2 (`KismetMathLibrary.ClampAngle` _returnvalue_pitch_2 -60.0 60.0) _returnvalue_yaw) 0.1)))))

(event `self.CapsuleComponent.OnComponentHit`
  (params (HitComponent :type "PrimitiveComponent Object Reference") (OtherActor :type "Actor Object Reference") (OtherComp :type "PrimitiveComponent Object Reference") (NormalImpulse :type "Vector Structure") (Hit :type "HitResult Structure (by ref)"))
  ;[1 1 1] On player hit
  (`self.GroundCheck`))

(event `self.ReceiveTick`
  (params (DeltaSeconds :type "Float (single-precision)"))
  ;[1 1 1] IK Placement
  (`self.AlignWithFloor`)
  (`self.ClampCamera`)
  (`self.CheckLocation`)
  (`self.RotateToVelocity`))

(event `AlignWithFloor`
  (bind _returnvalue (`self.K2_GetActorLocation`))
  (bind _capsulecomponent (`self.CapsuleComponent`))
  (bind _returnvalue_2 (`SceneComponent.K2_GetComponentRotation` _capsulecomponent))
  ;[1 1 1] Allign character rotation with floor
  (bind (_outhit _returnvalue_3) (`KismetSystemLibrary.LineTraceSingleForObjects` _returnvalue (- _returnvalue (0.0 0.0 100.0)) (`|MakeArray` "ObjectTypeQuery1" "ObjectTypeQuery4" "ObjectTypeQuery6" :!type "EObjectTypeQuery Enum") false (`|MakeArray` (`self.WaterSurface`) (`self.PhysicsVolume`) :!type "Actor Object Reference")))
  (if _returnvalue_3
    (bind (_bblockinghit _binitialoverlap _time _location _impactpoint _normal _impactnormal) (`GameplayStatics.BreakHitResult` _outhit))
    (`SceneComponent.K2_SetWorldRotation` _capsulecomponent (`KismetMathLibrary.RInterpTo` _returnvalue_2 (`KismetMathLibrary.MakeRotator` (.roll (`KismetMathLibrary.MakeRotFromXZ` (`SceneComponent.GetForwardVector` _capsulecomponent) _impactnormal)) (.pitch (`KismetMathLibrary.MakeRotFromYZ` (`SceneComponent.GetRightVector` _capsulecomponent) _impactnormal)) (.yaw _returnvalue_2)) (`GameplayStatics.GetWorldDeltaSeconds`) 10.0) true false)))

(event `self.ReceiveBeginPlay`
  (bind (_relativelocation_x _relativelocation_y _relativelocation_z) (`KismetMathLibrary.BreakVector` (`SceneComponent.RelativeLocation` (`self.Camera`))))
  ;[1 1 1] Assign Variables
  (bind _selfref (message `/Game/BluePrints/Interfaces/iControllerRefSystem.ControllerSelfRef` (`self.GetController`)))
  (set `self.ControllerRef` _selfref)
  (`KismetSystemLibrary.K2_SetTimerDelegate` (delegate `UnderwaterCheck`) 0.2 true)
  (bind _outactors (`GameplayStatics.GetAllActorsOfClass` "/Game/BluePrints/Character/OutOfWaterCamera.OutOfWaterCamera_C"))
  (for _array_element _outactors
    (set `self.OutOfWaterCamera` _array_element)
    (bind _outactors_2 (`GameplayStatics.GetAllActorsOfClass` "/Game/BluePrints/LevelObjects/WaterSurface.WaterSurface_C"))
    (for _array_element_2 _outactors_2
      (set `self.WaterSurface` _array_element_2)
      (bind _outactors_3 (`GameplayStatics.GetAllActorsOfClass` "/Script/Engine.PhysicsVolume"))
      (set `self.PhysicsVolume` (`|GetArrayItem` _outactors_3))
      (set `self.CameraOffsetToPlayer` _relativelocation_z)
      (set `self.StartingVector` (`self.K2_GetActorLocation`))
      (`KismetSystemLibrary.K2_SetTimer` null "UpdateFadeActors" 0.1 true)
      (bind _returnvalue (`KismetSystemLibrary.K2_SetTimerDelegate` (delegate `CheckCharactersPos`) 0.2 true))
      (set `self.UnderwaterCameraCheck` _returnvalue)
      (bind _asmy_game_instance (cast `/Game/BluePrints/MyGameInstance` (`GameplayStatics.GetGameInstance`)))
      (set `self.GameInstance` _asmy_game_instance))))

(event `CheckCharactersPos`
  (bind (_returnvalue_x _returnvalue_y _returnvalue_z) (`KismetMathLibrary.BreakVector` (`self.K2_GetActorLocation`)))
  (bind (_returnvalue_x_2 _returnvalue_y_2 _returnvalue_z_2) (`KismetMathLibrary.BreakVector` (`self.K2_GetActorLocation` (`self.WaterSurface`))))
  (bind _returnvalue (> _returnvalue_z _returnvalue_z_2))
  (bind _cutscene_ (message `/Game/BluePrints/Interfaces/iControllerRefSystem.ControllerHasCutscene?` (`self.ControllerRef`)))
  (if (not _cutscene_)
    (`self.SwapCamera` _returnvalue)
    (`self.UpdateFog` _returnvalue)))

(event `UnderwaterCheck`
  ;[1 1 1] Check if underwater
  (if (and (`self.Underwater?`) (`NavMovementComponent.IsFalling` (`self.CharacterMovement`)))
    (`ActorComponent.Activate` (`self.BubbleTrail`) false)
    (elif (not (`self.Underwater?`))
      (`ActorComponent.Deactivate` (`self.BubbleTrail`)))))

(event `GroundCheck`
  (bind _controllerref (`self.ControllerRef`))
  ;[1 1 1] Reset Jump if on ground
  (bind _returnvalue (`self.FloorDistanceCheck`))
  (if _returnvalue
    (message `/Game/BluePrints/Interfaces/iControllerFunctionSystem.SetJumpTrue` _controllerref)
    (`ActorComponent.Deactivate` (`self.BubbleTrail`))
    (message `/Game/BluePrints/Interfaces/iControllerFunctionSystem.SetIsJumpingFalse` _controllerref)
    (if (not (`self.Underwater?`))
      (`GameplayStatics.PlaySoundAtLocation` "/Game/Sound/TestSounds/UnderwaterThud.UnderwaterThud" (`self.K2_GetActorLocation`) (struct) (`/Game/BluePrints/MyGameInstance.AudioMasterVol` (`self.GameInstance`))))
    (else
      (message `/Game/BluePrints/Interfaces/iControllerFunctionSystem.SetJumpFalse` _controllerref))))

(event `/Game/BluePrints/Interfaces/IBaseMovment.ToggleCharacter`
  (bind _mesh (`self.Mesh`))
  (bind _charactermovement (`self.CharacterMovement`))
  (bind _controllerref (`self.ControllerRef`))
  (bind _capsulecomponent (`self.CapsuleComponent`))
  ;[1 1 1] Toggle character on and off
  (`/Engine/EditorBlueprintResources/StandardMacros.FlipFlop`
    (:`A`
      (`PrimitiveComponent.SetCollisionEnabled` _capsulecomponent "NoCollision")
      (`PrimitiveComponent.SetCollisionEnabled` (`self.Box`) "NoCollision")
      (`PrimitiveComponent.SetCollisionEnabled` _mesh "NoCollision")
      (`self.DisableInput` _controllerref)
      (set `self.IsDead` true)
      (`ActorComponent.ToggleActive` _charactermovement)
      (`KismetSystemLibrary.Delay` 0.5))
    (:`B`
      (`PrimitiveComponent.SetCollisionEnabled` _capsulecomponent "QueryAndPhysics")
      (`PrimitiveComponent.SetCollisionEnabled` (`self.Box`) "QueryAndPhysics")
      (`PrimitiveComponent.SetCollisionEnabled` _mesh "QueryOnly")
      (`self.EnableInput` _controllerref)
      (set `self.IsDead` false)
      (`ActorComponent.ToggleActive` _charactermovement)))
  (`SceneComponent.ToggleVisibility` (`self.Mesh`) false))

(event `Key|K`
  (params (Key :type "Key Structure"))
  ;[1 1 1] Damage Test
  (:`Pressed`
    (message `/Game/BluePrints/Interfaces/IBaseHealthChange.ChangeHealth` (`self.ControllerRef`) 1 true)))

(fn `CharacterBubbleTrailRef`
  (returns (ParticleSystem :type "ParticleSystemComponent Object Reference"))
  (return (`self.BubbleTrail`)))

(fn `CharacterClearCameraCheck`
  (returns (Complete :type Boolean))
  (bind _underwatercameracheck (`self.UnderwaterCameraCheck`))
  (if (`KismetSystemLibrary.K2_IsValidTimerHandle` _underwatercameracheck)
    (`KismetSystemLibrary.K2_ClearAndInvalidateTimerHandle` _underwatercameracheck)
    (return true)
    (else
      (return false))))

(fn `CharacterMovementRef`
  (returns (Movement :type "CharacterMovementComponent Object Reference"))
  (return (`self.CharacterMovement`)))

(fn `CharacterRootComponentRef`
  (returns (Root :type "SceneComponent Object Reference"))
  (return (`self.RootComponent`)))

(fn `CharacterSelfRef`
  (returns (CharacterRef :type "Character Object Reference"))
  (return self))

(fn `CharacterUnderWaterRef`
  (returns (`UnderWater?` :type Boolean))
  (return (`self.Underwater?`)))

(fn `DistanceCheck`
  (params (`X OffSet` :type "Float (double-precision)") (`Y OffSet` :type "Float (double-precision)") (`Z OffSet` :type "Float (double-precision)"))
  (returns (HasHit :type Boolean))
  (bind _returnvalue (`SceneComponent.K2_GetComponentLocation` (`self.CapsuleComponent`)))
  (bind (_outhit _returnvalue_2) (`KismetSystemLibrary.LineTraceSingleForObjects` _returnvalue (`KismetMathLibrary.MakeVector` (- (.x _returnvalue) `X OffSet`) (- (.y _returnvalue) `Y OffSet`) (- (.z _returnvalue) `Z OffSet`)) (`|MakeArray` "ObjectTypeQuery1" "ObjectTypeQuery4" "ObjectTypeQuery6" :!type "EObjectTypeQuery Enum") true (`|MakeArray` (`self.WaterSurface`) (`self.PhysicsVolume`) :!type "Actor Object Reference")))
  (bind _returnvalue_3 (`KismetMathLibrary.DegAcos` (`KismetMathLibrary.Dot_VectorVector` (`.ImpactNormal` (`GameplayStatics.BreakHitResult` _outhit)) (`KismetMathLibrary.Normal` (`KismetMathLibrary.GetRightVector` (struct))))))
  (return (and _returnvalue_2 (>= _returnvalue_3 40.0) (<= _returnvalue_3 150.0))))

(fn `FloorDistanceCheck`
  (returns (ReturnValue :type Boolean) (Location :type "Vector Structure"))
  (bind _hashit (`self.DistanceCheck` 0.0 0.0 (`self.FloorDistanceOffSet`)))
  (bind _hashit_2 (`self.DistanceCheck` 0.0 60.0 50.0))
  (bind _hashit_3 (`self.DistanceCheck` 0.0 -60.0 50.0))
  (bind _hashit_4 (`self.DistanceCheck` 0.0 60.0 25.0))
  (bind _hashit_5 (`self.DistanceCheck` 0.0 -60.0 25.0))
  (return (or _hashit _hashit_2 _hashit_3 _hashit_4 _hashit_5) (0.0 0.0 0.0)))

(fn `IKFootTrace`
  (params (TraceDistance :type "Float (double-precision)") (Socket :type Name))
  (returns (IKOffset :type "Float (double-precision)"))
  (bind (_returnvalue_x _returnvalue_y _returnvalue_z) (`KismetMathLibrary.BreakVector` (`self.K2_GetActorLocation`)))
  (bind (_returnvalue_x_2 _returnvalue_y_2) (`KismetMathLibrary.BreakVector` (`SceneComponent.GetSocketLocation` (`self.Mesh`) Socket)))
  (bind _returnvalue (`KismetMathLibrary.MakeVector` _returnvalue_x_2 _returnvalue_y_2 (- _returnvalue_z TraceDistance)))
  (bind (_outhit _returnvalue_2) (`KismetSystemLibrary.LineTraceSingle` :`Start` (`KismetMathLibrary.MakeVector` _returnvalue_x_2 _returnvalue_y_2 _returnvalue_z) :`End` _returnvalue :`TraceChannel` "TraceTypeQuery1" :`bTraceComplex` true :`DrawDebugType` "ForOneFrame"))
  (return (`KismetMathLibrary.SelectFloat` (/ (`KismetMathLibrary.VSize` (- _returnvalue (`.Location` (`GameplayStatics.BreakHitResult` _outhit)))) (`self.IKScale`)) 0.0 _returnvalue_2)))

(fn `IsCharacterDead`
  (returns (IsDead :type Boolean))
  (return (`self.IsDead`)))

(fn `SetHiddenMeshes`
  (bind _output_get (set `self.HiddenMeshes` (`self.HitMeshes`)))
  (for _array_element _output_get
    (for _array_element_2 (`self.K2_GetComponentsByClass` _array_element "/Game/BluePrints/BP_FadeComponent.BP_FadeComponent_C")
      (`/Game/BluePrints/BP_FadeComponent.ToggleHideMesh` _array_element_2 true))))

(fn `SetShownMeshes`
  (for _array_element (`self.HiddenMeshes`)
    (if (not (`KismetArrayLibrary.Array_Contains` (`self.HitMeshes`) _array_element))
      (for _array_element_2 (`self.K2_GetComponentsByClass` _array_element "/Game/BluePrints/BP_FadeComponent.BP_FadeComponent_C")
        (`/Game/BluePrints/BP_FadeComponent.ToggleHideMesh` _array_element_2 false)))))

(fn `SwapCamera`
  (params (`Underwater?` :type Boolean))
  (returns (Success :type Boolean))
  (if `Underwater?`
    (`PlayerController.SetViewTargetWithBlend` (`GameplayStatics.GetPlayerController` 0) (`self.OutOfWaterCamera`) 0.5 "VTBlend_Linear" 0.0 false)
    (else
      (`PlayerController.SetViewTargetWithBlend` (`GameplayStatics.GetPlayerController` 0) self 0.5 "VTBlend_Linear" 0.0 false)))
  (return true))

(fn `UpdateFadeActors`
  (bind _capsulecomponent (`self.CapsuleComponent`))
  (`KismetArrayLibrary.Array_Clear` (`self.HitMeshes`))
  (bind (_outhits _returnvalue) (`KismetSystemLibrary.CapsuleTraceMultiForObjects` (`SceneComponent.K2_GetComponentLocation` (`self.Camera`)) (`self.K2_GetActorLocation`) (`CapsuleComponent.CapsuleRadius` _capsulecomponent) (`CapsuleComponent.CapsuleHalfHeight` _capsulecomponent) (`|MakeArray` "ObjectTypeQuery1" :!type "EObjectTypeQuery Enum") false (`|MakeArray` (`self.WaterSurface`) (`self.PhysicsVolume`) :!type "Actor Object Reference")))
  (if _returnvalue
    (for _array_element _outhits
      (bind _asstatic_mesh_actor (cast `StaticMeshActor` (`.HitActor` (`GameplayStatics.BreakHitResult` _array_element))))
      (`KismetArrayLibrary.Array_AddUnique` (`self.HitMeshes`) _asstatic_mesh_actor)
      (`self.SetShownMeshes`)
      (`self.SetHiddenMeshes`))
    (else
      (`self.SetShownMeshes`))))

(fn `UpdateFog`
  (params (`Abovewater?` :type Boolean))
  (locals (FogDensity :type "Float (double-precision)"))
  (bind _outactors (`GameplayStatics.GetAllActorsOfClass` "/Script/Engine.ExponentialHeightFog"))
  (for _array_element _outactors
    (bind _output_get (set `self.UnderwaterFog` _array_element)))
  (`/Engine/EditorBlueprintResources/StandardMacros.IsValid` _output_get
    (:`Is Valid`
      (if `Abovewater?`
        (set `local.FogDensity` 0.0)
        (else
          (set `local.FogDensity` 0.05)))
      (`ExponentialHeightFogComponent.SetFogDensity` (`ExponentialHeightFog.Component` _output_get) (`local.FogDensity`))
      (return))))

(fn `UserConstructionScript`
  (set `self.IKScale` (.z (.scale (`self.GetTransform`))))
  (set `self.IKTraceDistance` (* (`CapsuleComponent.CapsuleHalfHeight` (`self.CapsuleComponent`)) (`self.IKScale`))))