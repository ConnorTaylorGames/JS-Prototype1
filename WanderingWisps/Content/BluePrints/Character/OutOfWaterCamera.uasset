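; OutOfWaterCamera is an actor that tracks the player's TestCharacter from above a referenced WaterSurface.
; BeginPlay caches the character and places the actor over it, a fixed height above the water.
; Each Tick takes X from the character's camera and Y from the character.
; Z follows at the same offset above the character, clamped so it never drops below that height over the water surface.
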(event `self.ReceiveBeginPlay`
  (bind _astest_character (cast `/Game/BluePrints/Character/TestCharacter` (`GameplayStatics.GetPlayerCharacter` 0)))
  (`/Engine/EditorBlueprintResources/StandardMacros.IsValid` _astest_character
    (:`Is Valid`
      (set `self.Character` _astest_character)
      (`self.K2_SetActorLocation` (`KismetMathLibrary.MakeVector` (.x (`self.K2_GetActorLocation` _astest_character)) (.y (`self.K2_GetActorLocation` _astest_character)) (+ (.z (`SceneComponent.K2_GetComponentLocation` (`StaticMeshActor.StaticMeshComponent` (`self.WaterSurface`)))) 500.0))))))

(event `self.ReceiveTick`
  (params (DeltaSeconds :type "Float (single-precision)"))
  (bind _character (`self.Character`))
  (`/Engine/EditorBlueprintResources/StandardMacros.IsValid` _character
    (:`Is Valid`
      (`self.K2_SetActorLocation` (`KismetMathLibrary.MakeVector` (.x (`SceneComponent.K2_GetComponentLocation` (`/Game/BluePrints/Character/TestCharacter.Camera` _character))) (.y (`self.K2_GetActorLocation` _character)) (`KismetMathLibrary.FClamp` (+ (.z (`self.K2_GetActorLocation` _character)) 500.0) (+ (.z (`SceneComponent.K2_GetComponentLocation` (`StaticMeshActor.StaticMeshComponent` (`self.WaterSurface`)))) 500.0) 10000000.0))))))

(fn `UserConstructionScript`)