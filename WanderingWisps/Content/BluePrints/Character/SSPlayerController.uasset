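; Player controller for a side-on character game with underwater sections, handling movement, jumping, pausing, health and death.
; Jumps launch the character, adding bubble trail and spray effects when underwater.
; Damage, optionally on a looping timer, respawns the player at the last checkpoint, or at zero health blends to an end camera and game-over widget.
; It also swaps out-of-water cameras and talks to the character through message calls.
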(event `AddPlayerHud`
  ;[0.1503 1 0] SETUP
  (bind _returnvalue (`|CreateWidget` "/Game/Widgets/PlayerHud.PlayerHud_C" self))
  (`UserWidget.AddToViewport` _returnvalue 0))

(event `self.ReceiveBeginPlay`
  ;[0.1503 1 0] SETUP
  ;;[1 1 1] Get player character and create UI
  (bind _characterref (message `/Game/BluePrints/Interfaces/iCharacterRefSystem.CharacterSelfRef` (`GameplayStatics.GetPlayerCharacter` 0)))
  (set `self.TestCharacter` _characterref)
  (bind _returnvalue (`GameplayStatics.GetCurrentLevelName` true))
  (if (not (`KismetStringLibrary.EqualEqual_StrStr` _returnvalue "MainMenuLevel"))
    (bind _asmy_game_instance (cast `/Game/BluePrints/MyGameInstance` (`GameplayStatics.GetGameInstance`)))
    (set `self.GameInstance` _asmy_game_instance)
    (bind _outactors (`GameplayStatics.GetAllActorsOfClass` "/Game/BluePrints/Character/OutOfWaterCamera.OutOfWaterCamera_C"))
    (for _array_element _outactors
      (set `self.OutOfWaterCamera` _array_element)
      (set `self.CanJump` false)
      (bind _outactors_2 (`GameplayStatics.GetAllActorsOfClass` "/Script/CinematicCamera.CineCameraActor"))
      (for _array_element_2 _outactors_2
        (if (`KismetStringLibrary.EqualEqual_StrStr` (`KismetSystemLibrary.GetDisplayName` _array_element_2) "EndCam")
          (set `self.EndCam` _array_element_2)
          (`self.SetupInitialSpawn` (`self.K2_GetActorLocation` (`self.TestCharacter`))))))))

(event `/Game/BluePrints/Interfaces/IBaseMovment.CharacterJump`
  (params (JumpDirection :type "Vector Structure"))
  ;[1 0.1687 0] INPUT EVENTS
  ;;[1 1 1] Character Jump
  (bind (_underwater_ _buubletrail _root _movement) (`self.GetCharcterRefsForJump`))
  (`Character.LaunchCharacter` (`self.TestCharacter`) JumpDirection false false)
  (if _underwater_
    (set `self.IsJumping?` true)
    (`ActorComponent.SetActive` _buubletrail true false)
    (if (not (`NavMovementComponent.IsFalling` _movement))
      (`GameplayStatics.SpawnEmitterAtLocation` "/Game/ParticleSystems/JumpSpray.JumpSpray" (`KismetMathLibrary.MakeVector` (.x (`SceneComponent.GetSocketLocation` _root "None")) (.y (`SceneComponent.GetSocketLocation` _root "None")) (- (.z (`SceneComponent.GetSocketLocation` _root "None")) (`self.FeetOffSet`))) (struct :`Roll` 180.0)))
    (else
      (set `self.IsJumping?` true))))

(event `InputAction|Jump`
  (params (Key :type "Key Structure"))
  ;[1 0.1687 0] INPUT EVENTS
  ;;[1 1 1] Press Space to jump
  (:`Pressed`
    (if (`self.CutScene?`)
      _
      (elif (`self.CanJump`)
        (set `self.CanJump` false)
        (`/Game/BluePrints/Character/TestCharacter.CharacterJump` (`self.StandardJump`))
        (`GameplayStatics.PlaySound2D` "/Game/Sound/TestSounds/character_dash.character_dash" (`/Game/BluePrints/MyGameInstance.AudioMasterVol` (`self.GameInstance`)))))))

(event `SetupInitialSpawn`
  (params (InitialSpawnPos :type "Vector Structure"))
  ;[0.1503 1 0] SETUP
  ;;[1 1 1] Setup initial spawn point
  (`self.SetCheckPoint` InitialSpawnPos))

(event `Key|LeftMouseButton`
  (params (Key :type "Key Structure"))
  ;[1 0.1687 0] INPUT EVENTS
  ;;[1 1 1] Refocus WIdget
  (:`Pressed`
    (`self.RefocusPlayerWidget`)))

(event `InputAction|Esc`
  (params (Key :type "Key Structure"))
  (bind _pausemenu (`self.PauseMenu`))
  (bind _tutorialpoint (`self.TutorialPoint`))
  ;[1 0.1687 0] INPUT EVENTS
  ;;[1 1 1] Pause Game
  (:`Pressed`
    (bind _returnvalue (`GameplayStatics.GetCurrentLevelName` true :!label _label))
    (if (`KismetStringLibrary.EqualEqual_StrStr` _returnvalue "MainMenuLevel")
      _
      (elif (`self.paused?`)
        (`/Engine/EditorBlueprintResources/StandardMacros.IsValid` _pausemenu
          (:`Is Valid`
            (`Widget.RemoveFromParent` _pausemenu)
            (`WidgetBlueprintLibrary.SetFocusToGameViewport`)
            (set `self.paused?` false)
            (`CharacterMovementComponent.SetMovementMode` (`Character.CharacterMovement` (`GameplayStatics.GetPlayerCharacter` 0)) "MOVE_Walking" 0)
            (`self.ShowHud`)))
        (else
          (set `self.paused?` true)
          (bind _returnvalue_2 (`|CreateWidget` "/Game/Widgets/PauseMenu.PauseMenu_C" self))
          (bind _output_get (set `self.PauseMenu` _returnvalue_2))
          (set `self.CurrentWidgetOnScreen` _returnvalue_2)
          (`UserWidget.AddToViewport` _output_get 0)
          (bind _resumebutton (`/Game/Widgets/PauseMenu.ResumeButton` _returnvalue_2))
          (`Widget.SetUserFocus` _resumebutton (`GameplayStatics.GetPlayerController` 0))
          (`Widget.SetKeyboardFocus` _resumebutton)
          (`CharacterMovementComponent.DisableMovement` (`Character.CharacterMovement` (`GameplayStatics.GetPlayerCharacter` 0)))
          (`/Engine/EditorBlueprintResources/StandardMacros.IsValid` _tutorialpoint
            (:`Is Valid`
              (message `/Game/BluePrints/Interfaces/iTutorialSystem.FadeText` _tutorialpoint))
            (:`Is Not Valid`
              _))
          (`GameplayStatics.PlaySound2D` "/Game/Sound/TestSounds/high_pitch_button.high_pitch_button" (`/Game/BluePrints/MyGameInstance.AudioMasterVol` (`self.GameInstance`)))
          (`self.HideHud`))))))

(event `/Game/BluePrints/Interfaces/iControllerRefSystem.ControllerSetTutorial`
  (params (TutorialPoint :type "Actor Object Reference"))
  ;[0.1503 1 0] SETUP
  ;;[1 1 1] Set Tutorial Point
  (set `self.TutorialPoint` TutorialPoint))

(event `Key|M`
  (params (Key :type "Key Structure"))
  ;[1 0.1687 0] INPUT EVENTS
  ;;[1 1 1] Pause Game
  ;;;[1 1 1] Test menu
  (:`Pressed`
    (goto _label)))

(event `HideHud`
  ;[1 0.1687 0] INPUT EVENTS
  (`Widget.RemoveFromParent` (`/Game/GameModes/PicnicGameMode.PlayerHud` (cast `/Game/GameModes/PicnicGameMode` (`GameplayStatics.GetGameMode`) :!pure true))))

(event `InputAxis|X_Movement`
  (params (AxisValue :type "Float (single-precision)"))
  (bind _testcharacter (`self.TestCharacter`))
  ;[1 0.1687 0] INPUT EVENTS
  ;;[1 1 1] PlayerMovement
  (if (not (`self.CutScene?`))
    (`/Engine/EditorBlueprintResources/StandardMacros.IsValid` _testcharacter
      (:`Is Valid`
        (`Pawn.AddMovementInput` _testcharacter (0.0 -1.0 0.0) AxisValue false)))))

(event `ShowHud`
  ;[1 0.1687 0] INPUT EVENTS
  (`UserWidget.AddToViewport` (`/Game/GameModes/PicnicGameMode.PlayerHud` (cast `/Game/GameModes/PicnicGameMode` (`GameplayStatics.GetGameMode`) :!pure true)) 0))

(event `InputAxis|Y_Movement`
  (params (AxisValue :type "Float (single-precision)"))
  (bind _testcharacter (`self.TestCharacter`))
  ;[1 0.1687 0] INPUT EVENTS
  ;;[1 1 1] PlayerMovement
  (if (not (`self.CutScene?`))
    (`/Engine/EditorBlueprintResources/StandardMacros.IsValid` _testcharacter
      (:`Is Valid`
        (set `CharacterMovementComponent.FallingLateralFriction` AxisValue (`Character.CharacterMovement` _testcharacter))))))

(event `self.StartTickHealth`
  (params (ChangeAmount :type Integer) (TickTime :type "Float (single-precision)") (IsDamage :type Boolean))
  ;[0 1 0.2767] HEALTH
  ;;[1 1 1] Tick Change Health
  (bind _returnvalue (`KismetSystemLibrary.K2_SetTimerDelegate` (delegate `Tick Damage`) TickTime true)))

(event `self.ChangeHealth`
  (params (ChangeAmount :type Integer) (IsDamage :type Boolean))
  (bind _currenthealth (`self.CurrentHealth`))
  ;[0 1 0.2767] HEALTH
  ;;[1 1 1] Change Health
  (`/Engine/EditorBlueprintResources/StandardMacros.IsValid` (`self.TestCharacter`)
    (:`Is Valid`
      (if IsDamage
        (bind _output_get (set `self.CurrentHealth` (- _currenthealth ChangeAmount)))
        (bind _isdead (`self.CheckIsDead` _output_get))
        (if _isdead
          (`self.DeathAnimation`
            (:`Exit`
              (`self.IsDead`)))
          (else
            (`self.GetCheckPoint`)))
        (else
          (bind _output_get_2 (set `self.CurrentHealth` (+ _currenthealth ChangeAmount)))
          (if (> _output_get_2 (`self.MaxHealth`))
            (set `self.CurrentHealth` (`self.MaxHealth`))))))))

(event `Tick Damage`
  ;[0 1 0.2767] HEALTH
  ;;[1 1 1] Tick Change Health
  (`self.ChangeHealth` (stale `self.StartTickHealth` ChangeAmount) (stale `self.StartTickHealth` IsDamage)))

(event `self.StopTickHealth`
  ;[0 1 0.2767] HEALTH
  ;;[1 1 1] Tick Change Health
  (`KismetSystemLibrary.K2_ClearAndInvalidateTimerHandle` (stale `self.StartTickHealth` _returnvalue)))

(event `self.GetCheckPoint`
  (bind _testcharacter (`self.TestCharacter`))
  (bind _returnvalue (`self.K2_GetActorLocation` _testcharacter))
  ;[1 0.8855 0] Checkpoint
  ;;[1 1 1] Set player to last checkPoint
  (message `/Game/BluePrints/Interfaces/IBaseMovment.ToggleCharacter` _testcharacter)
  (`GameplayStatics.PlaySoundAtLocation` "/Game/Sound/TestSounds/deathsounds2.deathsounds2" _returnvalue (struct) (`/Game/BluePrints/MyGameInstance.AudioMasterVol` (`self.GameInstance`)))
  (`GameplayStatics.SpawnEmitterAtLocation` "/Game/ParticleSystems/WispDeathEffect.WispDeathEffect" _returnvalue)
  (`KismetSystemLibrary.Delay` 1.5)
  (`self.K2_SetActorLocation` (`self.TestCharacter`) (`self.LastCheckPoint`) false true)
  (`GameplayStatics.PlaySound2D` "/Game/Sound/TestSounds/Player_Respawn_normal.Player_Respawn_normal" (`/Game/BluePrints/MyGameInstance.AudioMasterVol` (`self.GameInstance`)))
  (`KismetSystemLibrary.Delay` 2.3)
  (message `/Game/BluePrints/Interfaces/IBaseMovment.ToggleCharacter` (`self.TestCharacter`))
  (`GameplayStatics.SpawnEmitterAtLocation` "/Game/ParticleSystems/CollectibleExplosion.CollectibleExplosion" (`self.K2_GetActorLocation` (`self.TestCharacter`))))

(event `self.SetCheckPoint`
  (params (CheckPointLocation :type "Vector Structure"))
  ;[1 0.8855 0] Checkpoint
  ;;[1 1 1] Set players CheckPoint
  (set `self.LastCheckPoint` CheckPointLocation))

(fn `CheckIsDead`
  (params (CurrentHealth :type Integer))
  (returns (IsDead :type Boolean))
  (return (<= CurrentHealth 0)))

(fn `ControllerHasCutscene?`
  (returns (`Cutscene?` :type Boolean))
  (return (`self.CutScene?`)))

(fn `ControllerSelfRef`
  (returns (SelfRef :type "PlayerController Object Reference"))
  (return self))

(fn `GetCharcterRefsForJump`
  (returns (`UnderWater?` :type Boolean) (BuubleTrail :type "ParticleSystemComponent Object Reference") (Root :type "SceneComponent Object Reference") (Movement :type "CharacterMovementComponent Object Reference"))
  (bind _testcharacter (`self.TestCharacter`))
  (`|ExecutionSequence`
    (:`then_0`
      (bind _underwater_ (message `/Game/BluePrints/Interfaces/iCharacterRefSystem.CharacterUnderWaterRef` _testcharacter)))
    (:`then_1`
      (bind _particlesystem (message `/Game/BluePrints/Interfaces/iCharacterRefSystem.CharacterBubbleTrailRef` _testcharacter)))
    (:`then_2`
      (bind _root (message `/Game/BluePrints/Interfaces/iCharacterRefSystem.CharacterRootComponentRef` _testcharacter)))
    (:`then_3`
      (bind _movement (message `/Game/BluePrints/Interfaces/iCharacterRefSystem.CharacterMovementRef` _testcharacter)))
    (:`then_4`
      (return _underwater_ _particlesystem _root _movement))))

(fn `IsCharacterDead`
  (returns (IsDead :type Boolean))
  (return false))

(fn `IsDead`
  (bind _testcharacter (`self.TestCharacter`))
  (message `/Game/BluePrints/Interfaces/iCharacterRefSystem.CharacterClearCameraCheck` _testcharacter)
  (`self.K2_DestroyActor` _testcharacter)
  (`self.SetViewTargetWithBlend` (`GameplayStatics.GetPlayerController` 0) (`self.EndCam`) 0.0 "VTBlend_Linear" 0.0 false)
  (`Widget.RemoveFromParent` (`/Game/GameModes/PicnicGameMode.PlayerHud` (cast `/Game/GameModes/PicnicGameMode` (`GameplayStatics.GetGameMode`) :!pure true)))
  (bind _returnvalue (`|CreateWidget` "/Game/Widgets/GameOverWidget.GameOverWidget_C" self))
  (set `self.CurrentWidgetOnScreen` _returnvalue)
  (`UserWidget.AddToViewport` _returnvalue 0)
  (bind _replaybutton (`/Game/Widgets/GameOverWidget.ReplayButton` _returnvalue))
  (`Widget.SetUserFocus` _replaybutton self)
  (`Widget.SetKeyboardFocus` _replaybutton))

(fn `ResetCamera`
  (returns (`Sucess?` :type Boolean))
  (bind _returnvalue (`self.K2_GetPawn`))
  (`/Engine/EditorBlueprintResources/StandardMacros.IsValid` _returnvalue
    (:`Is Valid`
      (`self.SetViewTargetWithBlend` _returnvalue 0.7))))

(fn `SetIsJumpingFalse`
  (returns (Ignore :type Boolean))
  (set `self.IsJumping?` false)
  (return false))

(fn `SetJumpFalse`
  (returns (Ignore :type Boolean))
  (set `self.CanJump` false)
  (return false))

(fn `SetJumpTrue`
  (returns (Ignore :type Boolean))
  (set `self.CanJump` true)
  (return false))

(fn `ShowHidePawn`
  (params (`Hidden?` :type Boolean))
  (returns (HiddenOut :type Boolean))
  (bind _returnvalue (`self.K2_GetPawn`))
  (`self.SetActorHiddenInGame` _returnvalue `Hidden?`)
  (return (`Actor.bHidden` _returnvalue)))

(fn `SwapCamera`
  (params (`OutOfWater?` :type Boolean))
  (returns (`Success?` :type Boolean))
  (if `OutOfWater?`
    (`self.SetViewTargetWithBlend` (`self.OutOfWaterCamera`) 0.2 "VTBlend_Linear" 1000.0)
    (else
      (`self.SetViewTargetWithBlend` (`self.K2_GetPawn`) 0.2 "VTBlend_Linear" 1.0)))
  (return true))

(fn `UserConstructionScript`)