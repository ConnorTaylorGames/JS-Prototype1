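; Component that fades its owning StaticMeshActor's mesh, apparently when it hides the player from view.
; BeginPlay caches the slot 0 material, which must cast to a base Material, and creates a dynamic fade material instance.
; ToggleHideMesh swaps in that instance when hiding starts.
; Tick ramps a clamped fade value through a curve into the "Fade" parameter, restoring the original material once fully visible.
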(event `self.ReceiveBeginPlay`
  ;[1 1 1] Set Refereces
  (bind _asstatic_mesh_actor (cast `StaticMeshActor` (`self.GetOwner`)))
  (bind _output_get (set `self.ParentMesh` _asstatic_mesh_actor))
  (bind _asmaterial (cast `Material` (`PrimitiveComponent.GetMaterial` (`StaticMeshActor.StaticMeshComponent` _output_get) 0)))
  (set `self.BaseMaterial` _asmaterial)
  (bind _returnvalue (`KismetMaterialLibrary.CreateDynamicMaterialInstance` (`self.FadeMaterial`)))
  (set `self.FadeMaterialInst` _returnvalue))

(event `self.ReceiveTick`
  (params (DeltaSeconds :type "Float (single-precision)"))
  ;[1 1 1] Check if object is hiding player
  (set `self.DeltaTime` DeltaSeconds)
  (`/Engine/EditorBlueprintResources/StandardMacros.IsValid` (`self.ParentMesh`)
    (:`Is Valid`
      (if (`self.Hidden`)
        (set `self.currentFade` (`KismetMathLibrary.FClamp` (- (`self.currentFade`) (* (`self.DeltaTime`) (`self.FadeRate`))) 0.2))
        (else
          (set `self.currentFade` (`KismetMathLibrary.FClamp` (+ (`self.currentFade`) (* (`self.DeltaTime`) (`self.FadeRate`))) 0.2))))
      (`MaterialInstanceDynamic.SetScalarParameterValue` (`self.FadeMaterialInst`) "Fade" (`CurveFloat.GetFloatValue` (`self.FadeCurve`) (`self.currentFade`)))
      (if (and (== (`self.currentFade`) 1.0) (not (`self.Hidden`)))
        (`PrimitiveComponent.SetMaterial` (`StaticMeshActor.StaticMeshComponent` (`self.ParentMesh`)) 0 (`self.BaseMaterial`))))))

(fn `ToggleHideMesh`
  (params (Hidden :type Boolean))
  (if (!= Hidden (`self.Hidden`))
    (bind _output_get (set `self.Hidden` Hidden))
    (if _output_get
      (`PrimitiveComponent.SetMaterial` (`StaticMeshActor.StaticMeshComponent` (`self.ParentMesh`)) 0 (`self.FadeMaterialInst`)))))