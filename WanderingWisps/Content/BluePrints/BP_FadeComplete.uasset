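; Component for BP_DestructiblePlatform that fades the platform's destructible mesh out and back in, apparently when it hides the player.
; BeginPlay caches the owner's destructible and base material, and creates a dynamic instance of a fade material.
; ToggleHideMesh swaps in that instance when hiding starts.
; Tick ramps a clamped fade value through a curve into the "Fade" parameter, restoring the base material once fully visible.
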(event `self.ReceiveBeginPlay`
  ;[1 1 1] Set Refereces
  (bind _asbp_destructible_platform (cast `/Game/BluePrints/LevelObjects/Obstacles/BP_DestructiblePLatform` (`self.GetOwner`)))
  (bind _destructible (`/Game/BluePrints/LevelObjects/Obstacles/BP_DestructiblePLatform.Destructible` _asbp_destructible_platform))
  (set `self.DestructibleComp` _destructible)
  (bind _asmaterial (cast `Material` (`PrimitiveComponent.GetMaterial` _destructible 0)))
  (set `self.BaseMaterial` _asmaterial)
  (bind _returnvalue (`KismetMaterialLibrary.CreateDynamicMaterialInstance` (`self.FadeMaterial`)))
  (set `self.FadeMaterialInst` _returnvalue))

(event `self.ReceiveTick`
  (params (DeltaSeconds :type "Float (single-precision)"))
  ;[1 1 1] Check if object is hiding player
  (set `self.DeltaTime` DeltaSeconds)
  (`/Engine/EditorBlueprintResources/StandardMacros.IsValid` (`self.DestructibleComp`)
    (:`Is Valid`
      (if (`self.Hidden`)
        (set `self.currentFade` (`KismetMathLibrary.FClamp` (- (`self.currentFade`) (* (`self.DeltaTime`) (`self.FadeRate`)))))
        (else
          (set `self.currentFade` (`KismetMathLibrary.FClamp` (+ (`self.currentFade`) (* (`self.DeltaTime`) (`self.FadeRate`)))))))
      (`MaterialInstanceDynamic.SetScalarParameterValue` (`self.FadeMaterialInst`) "Fade" (`CurveFloat.GetFloatValue` (`self.FadeCurve`) (`self.currentFade`)))
      (if (and (== (`self.currentFade`) 1.0) (not (`self.Hidden`)))
        (`PrimitiveComponent.SetMaterial` (`self.DestructibleComp`) 0 (`self.BaseMaterial`))))))

(fn `ToggleHideMesh`
  (params (Hidden :type Boolean))
  (if (!= Hidden (`self.Hidden`))
    (bind _output_get (set `self.Hidden` Hidden))
    (if _output_get
      (`PrimitiveComponent.SetMaterial` (`self.DestructibleComp`) 0 (`self.FadeMaterialInst`)))))