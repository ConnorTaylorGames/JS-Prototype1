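; GuideToPoint is a guide actor that glides to a given target actor and destroys itself on arrival.
; SetNextPoint stores the target and starts a looping 0.01-second timer.
; Each tick blends the actor's full transform 1% toward the target's, giving an eased approach until locations match within a tiny tolerance.
; The computed Distance is never read, and a MoveToTargetTimeLine node is left unconnected.
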(event `/Game/BluePrints/Interfaces/iGuideToPointSystem.SetNextPoint`
  (params (NextPoint :type "Actor Object Reference"))
  (bind _output_get (set `self.NextPoint` NextPoint))
  (set `self.Distance` (`self.GetDistanceTo` _output_get))
  (`KismetSystemLibrary.K2_SetTimerDelegate` (delegate `Lerp`) 0.01 true))

(event `Lerp`
  (`self.K2_SetActorTransform` (`KismetMathLibrary.TLerp` (`self.GetTransform`) (`self.GetTransform` (`self.NextPoint`)) 0.01))
  (if (== (`self.K2_GetActorLocation` (`self.NextPoint`)) (`self.K2_GetActorLocation`))
    (`self.K2_DestroyActor`)))

(fn `UserConstructionScript`)