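; Level trigger point that shows a tutorial text widget when the player enters its box.
; A DoOnce gate precedes the player check; the player's overlap removes any ConflictingPoint widget, then creates and fades in this one.
; After ShowTime, a timer reverses the fade, then destroys the actor if it is not Replayable and the animation time check passes, otherwise resets the gate.
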(event `self.Box.OnComponentBeginOverlap`
  (params (OverlappedComponent :type "PrimitiveComponent Object Reference") (OtherActor :type "Actor Object Reference") (OtherComp :type "PrimitiveComponent Object Reference") (OtherBodyIndex :type Integer) (bFromSweep :type Boolean) (SweepResult :type "HitResult Structure (by ref)"))
  (bind _tutorial (`self.Tutorial`))
  (bind _conflictingpoint (`self.ConflictingPoint`))
  (`/Engine/EditorBlueprintResources/StandardMacros.DoOnce` false :!label _label
    (:`Completed`
      (if (== OtherActor (`GameplayStatics.GetPlayerCharacter` 0))
        (`/Engine/EditorBlueprintResources/StandardMacros.IsValid` _conflictingpoint
          (:`Is Valid`
            (`Widget.RemoveFromParent` (`/Game/BluePrints/LevelObjects/TutorialPoint.Tutorial` _conflictingpoint)))
          (:`Is Not Valid`
            _))
        (bind _returnvalue (`|CreateWidget` "/Game/Widgets/TutorialWidget.TutorialWidget_C" (`GameplayStatics.GetPlayerController` 0)))
        (bind _output_get (set `self.Tutorial` _returnvalue))
        (set `/Game/Widgets/TutorialWidget.TutorialText` (`self.TutorialText`) _output_get)
        (`UserWidget.AddToViewport` _returnvalue 0)
        (`UserWidget.PlayAnimation` _tutorial (`/Game/Widgets/TutorialWidget.Fade` _tutorial) 0.0 1 "Forward" 1.0)
        (`KismetSystemLibrary.K2_SetTimerDelegate` (delegate `FadeWidget`) (`self.ShowTime`))))))

(event `FadeWidget`
  (bind _tutorial (`self.Tutorial`))
  (bind _fade (`/Game/Widgets/TutorialWidget.Fade` _tutorial))
  (`UserWidget.PlayAnimation` _tutorial _fade 0.0 1 "Reverse" 1.0)
  (if (and (<= (`UserWidget.GetAnimationCurrentTime` _tutorial _fade) 0.6) (not (`self.Replayable?`)))
    (`self.K2_DestroyActor`)
    (else
      (goto _label :!via `Reset`))))

(fn `UserConstructionScript`)