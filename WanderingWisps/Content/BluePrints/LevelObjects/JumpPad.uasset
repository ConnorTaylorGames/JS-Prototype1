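; JumpPad is a level-object Blueprint that launches an overlapping player character using a JumpBoost value.
; On BeginPlay it creates a dynamic material on the Cube and sets a blue emissive colour.
; Box overlaps are validated through a character self-reference message, then send CharacterJumpMessage to the instigator's controller, which receives the boost.
; A DoOnce blocks repeat launches until a short delay resets the pad.
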(event `self.ReceiveBeginPlay`
  (bind _returnvalue (`PrimitiveComponent.CreateDynamicMaterialInstance` (`self.Cube`) 0 "/Game/Assets/Enviroment/Objects/Traps/PressurePlate/PressurePlateMat.PressurePlateMat"))
  (`MaterialInstanceDynamic.SetVectorParameterValue` _returnvalue "EmissiveColour" (struct :`G` 0.436636 :`B` 0.776042 :`A` 1.0)))

(event `self.Box.OnComponentBeginOverlap`
  (params (OverlappedComponent :type "PrimitiveComponent Object Reference") (OtherActor :type "Actor Object Reference") (OtherComp :type "PrimitiveComponent Object Reference") (OtherBodyIndex :type Integer) (bFromSweep :type Boolean) (SweepResult :type "HitResult Structure (by ref)"))
  ;[1 1 1] Launch player character
  (`self.IsCharacterValid` OtherActor
    (:`Exit`
      (`/Engine/EditorBlueprintResources/StandardMacros.DoOnce` false :!label _label
        (:`Completed`
          (message `/Game/BluePrints/Interfaces/IBaseMovment.CharacterJump` (`Pawn.GetController` (`Actor.Instigator` OtherActor)) (`self.JumpBoost`))
          (`KismetSystemLibrary.Delay` 0.5)
          (`self.ResetJumpPad`))))))

(event `ResetJumpPad`
  ;[1 1 1] Launch player character
  (goto _label :!via `Reset`))

(fn `UserConstructionScript`)