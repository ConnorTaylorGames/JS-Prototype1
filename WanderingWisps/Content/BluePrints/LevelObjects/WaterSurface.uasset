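; Water surface level actor that handles the player's transition into and out of water, with splash, ambient sound and depth-based lighting.
; Box overlaps toggle the character's underwater state and camera, then looping timers poll camera height against the surface to switch sounds.
; Surface mesh overlap spawns the splash.
; Another timer drives light bloom and intensity from surface and player heights, while a GameInstance dispatcher updates audio volume.
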(event `UpdateAudio`
  ;[1 1 1] Vol System
  (`AudioComponent.SetVolumeMultiplier` (`self.Audio`) (`/Game/BluePrints/MyGameInstance.AudioMasterVol` (`self.GameInstance`))))

(event `self.ReceiveBeginPlay`
  (bind _returnvalue (`GameplayStatics.GetPlayerCharacter` 0))
  ;[1 1 1] BeginPlay
  (`/Engine/EditorBlueprintResources/StandardMacros.IsValid` _returnvalue
    (:`Is Valid`
      (bind _astest_character (cast `/Game/BluePrints/Character/TestCharacter` _returnvalue))
      (set `self.Character` _astest_character)
      (`AudioComponent.SetSound` (`self.Audio`) (`|GetArrayItem` (`self.WorldSounds`)))
      (bind _asmy_game_instance (cast `/Game/BluePrints/MyGameInstance` (`GameplayStatics.GetGameInstance`)))
      (bind _output_get (set `self.GameInstance` _asmy_game_instance))
      (add `/Game/BluePrints/MyGameInstance.UpdateAudioEventDispatcher` _output_get (`|CreateDelegate` :!event `UpdateAudio`))
      (bind _returnvalue_2 (`KismetSystemLibrary.K2_SetTimerDelegate` (delegate `DepthLighting`) 0.2 true))
      (set `self.DepthLightingHandle` _returnvalue_2))))

(event `DepthLighting`
  (bind _character (`self.Character`))
  (bind (_returnvalue_x _returnvalue_y _returnvalue_z) (`KismetMathLibrary.BreakVector` (`SceneComponent.K2_GetComponentLocation` (`self.StaticMeshComponent`))))
  (bind (_returnvalue_x_2 _returnvalue_y_2 _returnvalue_z_2) (`KismetMathLibrary.BreakVector` (`SceneComponent.K2_GetComponentLocation` (`Character.CapsuleComponent` _character))))
  (bind _returnvalue (+ _returnvalue_z _returnvalue_z_2))
  ;[1 1 1] Change lighting effects based on depth
  (`/Engine/EditorBlueprintResources/StandardMacros.IsValid` _character
    (:`Is Valid`
      (`LightComponent.SetBloomScale` (`/Game/BluePrints/LevelObjects/LightingTest.DirectionalLight1` (`self.LightActor`)) (`self.ClampToDivision` _returnvalue 0.0 3600.0 1000.0))
      (`LightComponent.SetIntensity` (`Light.LightComponent` (`self.DirectionalLightActor`)) (`self.ClampToDivision` _returnvalue 0.0 4000.0 1000.0)))
    (:`Is Not Valid`
      (`KismetSystemLibrary.K2_ClearAndInvalidateTimerHandle` (`self.DepthLightingHandle`)))))

(event `self.StaticMeshComponent.OnComponentBeginOverlap`
  (params (OverlappedComponent :type "PrimitiveComponent Object Reference") (OtherActor :type "Actor Object Reference") (OtherComp :type "PrimitiveComponent Object Reference") (OtherBodyIndex :type Integer) (bFromSweep :type Boolean) (SweepResult :type "HitResult Structure (by ref)"))
  (bind _z (.z (`SceneComponent.K2_GetComponentLocation` (`self.StaticMeshComponent`))))
  (bind _returnvalue (`KismetMathLibrary.MakeVector` (.x (`.Location` (`GameplayStatics.BreakHitResult` SweepResult))) (.y (`.Location` (`GameplayStatics.BreakHitResult` SweepResult))) _z))
  ;[1 1 1] Spawn water splash when player leaves the water
  (if (== OtherActor (`self.Character`))
    (if (!= _returnvalue (`KismetMathLibrary.MakeVector` 0.0 0.0 _z))
      (`GameplayStatics.SpawnEmitterAtLocation` "/Game/ParticleSystems/WaterSplash.WaterSplash" _returnvalue))))

(event `self.Box.OnComponentBeginOverlap`
  (params (OverlappedComponent :type "PrimitiveComponent Object Reference") (OtherActor :type "Actor Object Reference") (OtherComp :type "PrimitiveComponent Object Reference") (OtherBodyIndex :type Integer) (bFromSweep :type Boolean) (SweepResult :type "HitResult Structure (by ref)"))
  ;[1 1 1] Player Enters water
  (if (== OtherActor (`GameplayStatics.GetPlayerCharacter` 0))
    (bind _astest_character (cast `/Game/BluePrints/Character/TestCharacter` OtherActor))
    (bind _output_get (set `/Game/BluePrints/Character/TestCharacter.Underwater?` true _astest_character))
    (`/Game/BluePrints/Character/TestCharacter.SwapCamera` _astest_character _output_get)
    (bind _returnvalue (`KismetSystemLibrary.K2_SetTimerDelegate` (delegate `IsCameraBelowWater?`) 0.2 true))))

(event `IsCameraBelowWater?`
  (bind (_returnvalue_x _returnvalue_y _returnvalue_z) (`KismetMathLibrary.BreakVector` (`SceneComponent.K2_GetComponentLocation` (`self.StaticMeshComponent`))))
  (bind (_returnvalue_x_2 _returnvalue_y_2 _returnvalue_z_2) (`KismetMathLibrary.BreakVector` (`SceneComponent.K2_GetComponentLocation` (`/Game/BluePrints/Character/TestCharacter.Camera` (`self.Character`)))))
  ;[1 1 1] Camera Enters Water
  (if (<= _returnvalue_z_2 _returnvalue_z)
    (`AudioComponent.SetSound` (`self.Audio`) (`|GetArrayItem` (`self.WorldSounds`)))
    (`KismetSystemLibrary.K2_ClearAndInvalidateTimerHandle` (stale `self.Box.OnComponentBeginOverlap` _returnvalue))))

(event `self.Box.OnComponentEndOverlap`
  (params (OverlappedComponent :type "PrimitiveComponent Object Reference") (OtherActor :type "Actor Object Reference") (OtherComp :type "PrimitiveComponent Object Reference") (OtherBodyIndex :type Integer))
  ;[1 1 1] Player Leaves Water
  (if (== OtherActor (`GameplayStatics.GetPlayerCharacter` 0))
    (bind _astest_character (cast `/Game/BluePrints/Character/TestCharacter` OtherActor))
    (bind _output_get (set `/Game/BluePrints/Character/TestCharacter.Underwater?` false _astest_character))
    (`/Game/BluePrints/Character/TestCharacter.SwapCamera` _astest_character _output_get)
    (bind _returnvalue (`KismetSystemLibrary.K2_SetTimerDelegate` (delegate `IsCameraAboveWater`) 0.2 true))))

(event `IsCameraAboveWater`
  (bind (_returnvalue_x _returnvalue_y _returnvalue_z) (`KismetMathLibrary.BreakVector` (`SceneComponent.K2_GetComponentLocation` (`self.StaticMeshComponent`))))
  (bind (_returnvalue_x_2 _returnvalue_y_2 _returnvalue_z_2) (`KismetMathLibrary.BreakVector` (`SceneComponent.K2_GetComponentLocation` (`/Game/BluePrints/Character/TestCharacter.Camera` (`self.Character`)))))
  ;[1 1 1] Camera Leaves Water
  (if (>= _returnvalue_z_2 _returnvalue_z)
    (`AudioComponent.SetSound` (`self.Audio`) (`|GetArrayItem` (`self.WorldSounds`) 1))
    (`KismetSystemLibrary.K2_ClearAndInvalidateTimerHandle` (stale `self.Box.OnComponentEndOverlap` _returnvalue))))

(fn `UserConstructionScript`)