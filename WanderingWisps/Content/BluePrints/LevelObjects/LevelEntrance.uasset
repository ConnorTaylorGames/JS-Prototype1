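; Level entrance actor for a cave with a stone door and portal, apparently meant to open once all collectables are gathered.
; RaiseDoor and BeginPlay are empty; the door sequence and collision-disable nodes are disconnected, so they never run.
; That unwired sequence activates portal and particles, plays a sound, moves the door vertically by Timeline, then restores collision.
; CheckIfPlayerWon returns true when the passed Collectables count is zero or less.
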(event `RaiseDoor`
  ;[1 1 1] Raise the door
)

(event `self.ReceiveBeginPlay`
  ;[1 1 1] Setup Manager
)

(fn `CheckIfPlayerWon`
  (params (Collectables :type Integer))
  (returns (`Winner?` :type Boolean))
  (return (<= Collectables 0)))

(fn `UserConstructionScript`)