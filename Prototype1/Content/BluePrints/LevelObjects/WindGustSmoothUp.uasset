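; Wind gust level object that smoothly pushes the player character with a configurable force while inside its box volume.
; Overlap starts a fast looping timer that adds force to character movement, and leaving clears it.
; If marked Triggered, it starts with the bubble stream hidden and collision off until SwitchActivated enables both.
; Its audio replays continuously and follows the game instance's master volume through an event dispatcher.
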(event `Activate Fan`
  ;[1 1 1] Activate fan on pressure plate
)

(event `self.ReceiveBeginPlay`
  ;[1 1 1] Begin
  (bind _asmy_game_instance (cast `/Game/BluePrints/MyGameInstance` (`GameplayStatics.GetGameInstance`)))
  (bind _output_get (set `self.GameInstance` _asmy_game_instance))
  (add `/Game/BluePrints/MyGameInstance.UpdateAudioEventDispatcher` _output_get (delegate `UpdateAudio`))
  (`self.PlayAudio`)
  (if (`self.Triggered?`)
    (`SceneComponent.SetHiddenInGame` (`self.BubbleStream`) true false)
    (`PrimitiveComponent.SetCollisionEnabled` (`self.Box`) "NoCollision")))

(event `self.Audio.OnAudioFinished`
  ;[1 1 1] Replay audio when finished
  (`self.PlayAudio`))

(event `PlayAudio`
  (bind _audio (`self.Audio`))
  ;[1 1 1] Play audio
  (`AudioComponent.SetVolumeMultiplier` _audio (`/Game/BluePrints/MyGameInstance.AudioMasterVol` (`self.GameInstance`)))
  (`AudioComponent.Play` _audio 0.0))

(event `UpdateAudio`
  ;[1 1 1] update the volume of the audio
  (`AudioComponent.SetVolumeMultiplier` (`self.Audio`) (`/Game/BluePrints/MyGameInstance.AudioMasterVol` (`self.GameInstance`))))

(event `LiftPlayer`
  ;[1 1 1] Lift Player Timer
  (if (`self.InsideWind`)
    (`CharacterMovementComponent.AddForce` (`Character.CharacterMovement` (`self.Player`)) (`self.Force DIrection`))))

(event `self.Box.OnComponentBeginOverlap`
  (params (OverlappedComponent :type "PrimitiveComponent Object Reference") (OtherActor :type "Actor Object Reference") (OtherComp :type "PrimitiveComponent Object Reference") (OtherBodyIndex :type Integer) (bFromSweep :type Boolean) (SweepResult :type "HitResult Structure (by ref)"))
  (bind (_astest_character _bsuccess) (cast `/Game/BluePrints/Character/TestCharacter` OtherActor :!pure true))
  ;[1 1 1] Begin Overlap
  (`/Engine/EditorBlueprintResources/StandardMacros.IsValid` OtherActor
    (:`Is Valid`
      (if _bsuccess
        (set `self.Player` _astest_character)
        (set `self.InsideWind` true)
        (bind _returnvalue (`KismetSystemLibrary.K2_SetTimerDelegate` (delegate `LiftPlayer`) 0.01 true))
        (bind _output_get (set `self.PlayerLiftTimer` _returnvalue))))))

(event `self.Box.OnComponentEndOverlap`
  (params (OverlappedComponent :type "PrimitiveComponent Object Reference") (OtherActor :type "Actor Object Reference") (OtherComp :type "PrimitiveComponent Object Reference") (OtherBodyIndex :type Integer))
  ;[1 1 1] End Overlap
  (`/Engine/EditorBlueprintResources/StandardMacros.IsValid` OtherActor
    (:`Is Valid`
      (if (== OtherActor (`self.Player`))
        (set `self.InsideWind` false)
        (`KismetSystemLibrary.K2_ClearAndInvalidateTimerHandle` (stale `self.Box.OnComponentBeginOverlap` _output_get))))))

(fn `SwitchActivated`
  (returns (`Activated?` :type Boolean))
  (`SceneComponent.SetHiddenInGame` (`self.BubbleStream`) false false)
  (`PrimitiveComponent.SetCollisionEnabled` (`self.Box`) "QueryAndPhysics")
  (return true))

(fn `UserConstructionScript`)