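; WinZone is a level trigger that ends the game with a win when the player enters it with no collectables remaining.
; At BeginPlay it caches the ScoreManager actor found in the level.
; On box overlap with the player character, it passes the manager's score to CheckIfPlayerWon, which succeeds at zero or below.
; A win disables TestCharacter movement, displays the WinnerBP widget and shows the mouse cursor.
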(event `self.ReceiveBeginPlay`
  ;[1 1 1] Setup Manager
  (bind _outactors (`GameplayStatics.GetAllActorsOfClass` "/Game/BluePrints/Managers/ScoreManager.ScoreManager_C"))
  (for _array_element _outactors
    (set `self.ScoreManager` _array_element)))

(event `self.Box.OnComponentBeginOverlap`
  (params (OverlappedComponent :type "PrimitiveComponent Object Reference") (OtherActor :type "Actor Object Reference") (OtherComp :type "PrimitiveComponent Object Reference") (OtherBodyIndex :type Integer) (bFromSweep :type Boolean) (SweepResult :type "HitResult Structure (by ref)"))
  (bind _returnvalue (`GameplayStatics.GetPlayerController` 0))
  (bind _returnvalue_2 (`GameplayStatics.GetPlayerCharacter` 0))
  (bind (_astest_character _bsuccess) (cast `/Game/BluePrints/Character/TestCharacter` _returnvalue_2 :!pure true))
  ;[1 1 1] On Colision check if player has won and react accordingly
  (if (== OtherActor _returnvalue_2)
    (bind _no__collectables (`/Game/BluePrints/Managers/ScoreManager.ReturnScore` (`self.ScoreManager`)))
    (bind _winner_ (`self.CheckIfPlayerWon` _no__collectables))
    (if _winner_
      (if _bsuccess
        (`CharacterMovementComponent.DisableMovement` (`Character.CharacterMovement` _astest_character))
        (bind _returnvalue_3 (`|CreateWidget` "/Game/Widgets/WinnerBP.WinnerBP_C" _returnvalue))
        (`UserWidget.AddToViewport` _returnvalue_3 0)
        (set `PlayerController.bShowMouseCursor` true _returnvalue)))))

(fn `CheckIfPlayerWon`
  (params (Collectables :type Integer))
  (returns (`Winner?` :type Boolean))
  (return (<= Collectables 0)))

(fn `UserConstructionScript`)