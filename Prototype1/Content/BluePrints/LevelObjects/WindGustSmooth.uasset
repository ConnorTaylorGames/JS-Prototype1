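; A wind gust level object that pushes the player character upward while they stand inside its box volume.
; Box overlaps store the TestCharacter as Player and toggle an InsideWind flag, and Tick applies a constant upward force through its CharacterMovement while that flag is set.
; When Triggered, it starts with the gust visuals hidden and collision off until ActivateFan re-enables both.
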(event `Activate Fan`
  (`SceneComponent.SetHiddenInGame` (`self.WindGusts`) false false)
  (`PrimitiveComponent.SetCollisionEnabled` (`self.Box`) "QueryAndPhysics"))

(event `self.ReceiveBeginPlay`
  (if (`self.Triggered?`)
    (`SceneComponent.SetHiddenInGame` (`self.WindGusts`) true false)
    (`PrimitiveComponent.SetCollisionEnabled` (`self.Box`) "NoCollision")))

(event `self.ReceiveTick`
  (params (DeltaSeconds :type "Float (single-precision)"))
  (if (`self.InsideWind`)
    (`CharacterMovementComponent.AddForce` (`Character.CharacterMovement` (`self.Player`)) (0.0 0.0 15000.0))))

(event `self.Box.OnComponentBeginOverlap`
  (params (OverlappedComponent :type "PrimitiveComponent Object Reference") (OtherActor :type "Actor Object Reference") (OtherComp :type "PrimitiveComponent Object Reference") (OtherBodyIndex :type Integer) (bFromSweep :type Boolean) (SweepResult :type "HitResult Structure (by ref)"))
  (bind (_astest_character _bsuccess) (cast `/Game/BluePrints/Character/TestCharacter` OtherActor :!pure true))
  (`/Engine/EditorBlueprintResources/StandardMacros.IsValid` OtherActor
    (:`Is Valid`
      (if _bsuccess
        (set `self.Player` _astest_character)
        (set `self.InsideWind` true)))))

(event `self.Box.OnComponentEndOverlap`
  (params (OverlappedComponent :type "PrimitiveComponent Object Reference") (OtherActor :type "Actor Object Reference") (OtherComp :type "PrimitiveComponent Object Reference") (OtherBodyIndex :type Integer))
  (`/Engine/EditorBlueprintResources/StandardMacros.IsValid` OtherActor
    (:`Is Valid`
      (if (== OtherActor (`self.Player`))
        (set `self.InsideWind` false)))))

(fn `UserConstructionScript`)