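; TestCharacter is a test character Blueprint that relies on SSPlayerController for jump state and health.
; It caches the cast controller on BeginPlay.
; On capsule hits, a downward WorldStatic line trace from the capsule's location checks for floor within an offset and, if found, calls SetJumping on the controller to reset the jump.
; A debug K key applies damage through the controller's ChangeHealth.
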(event `self.ReceiveBeginPlay`
  ;[1 1 1] Get Contoller
  (bind _asssplayer_controller (cast `/Game/BluePrints/Character/SSPlayerController` (`self.GetController`)))
  (set `self.ControllerRef` _asssplayer_controller))

(event `self.CapsuleComponent.OnComponentHit`
  (params (HitComponent :type "PrimitiveComponent Object Reference") (OtherActor :type "Actor Object Reference") (OtherComp :type "PrimitiveComponent Object Reference") (NormalImpulse :type "Vector Structure") (Hit :type "HitResult Structure (by ref)"))
  ;[1 1 1] Reset Jump of in ground
  (bind _returnvalue (`self.FloorDistanceCheck`))
  (if _returnvalue
    (`/Game/BluePrints/Character/SSPlayerController.SetJumping` (`self.ControllerRef`))))

(event `Key|K`
  (params (Key :type "Key Structure"))
  ;[1 1 1] Damage Test
  (:`Pressed`
    (`/Game/BluePrints/Interfaces/IBaseHealthChange.ChangeHealth` (`self.ControllerRef`) 1 true)))

(fn `FloorDistanceCheck`
  (returns (ReturnValue :type Boolean) (Location :type "Vector Structure"))
  (bind _returnvalue (`SceneComponent.K2_GetComponentLocation` (`self.CapsuleComponent`)))
  (bind (_outhit _returnvalue_2) (`KismetSystemLibrary.LineTraceSingleForObjects` _returnvalue (`KismetMathLibrary.MakeVector` (.x _returnvalue) (.y _returnvalue) (- (.z _returnvalue) (`self.FloorDistanceOffSet`))) (`|MakeArray` "ObjectTypeQuery1" :!type "EObjectTypeQuery Enum")))
  (return _returnvalue_2 (`.Location` (`GameplayStatics.BreakHitResult` _outhit))))

(fn `UserConstructionScript`)