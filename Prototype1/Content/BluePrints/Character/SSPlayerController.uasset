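; Player controller that creates the HUD and handles side-to-side movement, jumping, health, checkpoints and pausing for TestCharacter.
; Jumps launch the character and stay locked until SetJumping re-arms them.
; Non-lethal damage teleports the character to the last checkpoint, death destroys it and shows game over, and a looping timer can repeat health changes.
; Esc or a test M key opens the pause menu and pauses the game.
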(event `InputAction|Esc`
  (params (Key :type "Key Structure"))
  ;[1 1 1] Pause Game
  (:`Pressed`
    (bind _returnvalue (`|CreateWidget` "/Game/Widgets/PauseMenu.PauseMenu_C" self :!label _label))
    (`UserWidget.AddToViewport` _returnvalue 0)
    (set `self.bShowMouseCursor` true)
    (`GameplayStatics.SetGamePaused` true)
    (`GameplayStatics.PlaySound2D` "/Game/Sound/TestSounds/high_pitch_button.high_pitch_button" (`/Game/BluePrints/MyGameInstance.AudioMasterVol` (`self.GameInstance`)))))

(event `Key|M`
  (params (Key :type "Key Structure"))
  ;[1 1 1] Pause Game
  ;;[1 1 1] Test menu
  (:`Pressed`
    (goto _label)))

(event `self.ReceiveBeginPlay`
  ;[1 1 1] Get player character and create UI
  (set `self.TestCharacter` (cast `/Game/BluePrints/Character/TestCharacter` (`GameplayStatics.GetPlayerCharacter` 0) :!pure true))
  (bind _returnvalue (`|CreateWidget` "/Game/Widgets/PlayerHud.PlayerHud_C" self))
  (`UserWidget.AddToViewport` _returnvalue 0)
  (bind _asmy_game_instance (cast `/Game/BluePrints/MyGameInstance` (`GameplayStatics.GetGameInstance`)))
  (set `self.GameInstance` _asmy_game_instance))

(event `InputAxis|K_Movement`
  (params (AxisValue :type "Float (single-precision)"))
  (bind _testcharacter (`self.TestCharacter`))
  ;[1 1 1] Left and Right Movement
  (`/Engine/EditorBlueprintResources/StandardMacros.IsValid` _testcharacter
    (:`Is Valid`
      (`Pawn.AddMovementInput` _testcharacter (`self.GetActorRightVector` _testcharacter) AxisValue false))))

(event `InputAction|Jump`
  (params (Key :type "Key Structure"))
  ;[1 1 1] Press Space to jump
  (:`Pressed`
    (if (`self.CanJump`)
      (`/Game/BluePrints/Character/TestCharacter.CharacterJump` (`self.StandardJump`))
      (set `self.CanJump` false))))

(event `/Game/BluePrints/Interfaces/IBaseMovment.CharacterJump`
  (params (JumpDirection :type "Vector Structure"))
  ;[1 1 1] Character Jump
  (`Character.LaunchCharacter` (`self.TestCharacter`) JumpDirection false false))

(event `self.ChangeHealth`
  (params (ChangeAmount :type Integer) (IsDamage :type Boolean))
  (bind _currenthealth (`self.CurrentHealth`))
  ;[1 1 1] Change Health
  (`/Engine/EditorBlueprintResources/StandardMacros.IsValid` (`self.TestCharacter`)
    (:`Is Valid`
      (if IsDamage
        (bind _output_get (set `self.CurrentHealth` (- _currenthealth ChangeAmount)))
        (bind _isdead (`self.CheckIsDead` _output_get))
        (if _isdead
          (`self.IsDead`)
          (else
            (`self.GetCheckPoint`)))
        (else
          (bind _output_get_2 (set `self.CurrentHealth` (+ _currenthealth ChangeAmount)))
          (if (> _output_get_2 (`self.MaxHealth`))
            (set `self.CurrentHealth` (`self.MaxHealth`))))))))

(event `self.StartTickHealth`
  (params (ChangeAmount :type Integer) (TickTime :type "Float (single-precision)") (IsDamage :type Boolean))
  ;[1 1 1] Tick Change Health
  (bind _returnvalue (`KismetSystemLibrary.K2_SetTimerDelegate` (delegate `Tick Damage`) TickTime true)))

(event `Tick Damage`
  ;[1 1 1] Tick Change Health
  (`self.ChangeHealth` (stale `self.StartTickHealth` ChangeAmount) (stale `self.StartTickHealth` IsDamage)))

(event `self.StopTickHealth`
  ;[1 1 1] Tick Change Health
  (`KismetSystemLibrary.K2_ClearAndInvalidateTimerHandle` (stale `self.StartTickHealth` _returnvalue)))

(event `self.SetCheckPoint`
  (params (CheckPointLocation :type "Vector Structure"))
  ;[1 1 1] Set players CheckPoint
  (set `self.LastCheckPoint` CheckPointLocation))

(event `self.GetCheckPoint`
  ;[1 1 1] Set player to last checkPoint
  (`self.K2_SetActorLocation` (`self.TestCharacter`) (`self.LastCheckPoint`) false true))

(fn `CheckIsDead`
  (params (CurrentHealth :type Integer))
  (returns (IsDead :type Boolean))
  (return (<= CurrentHealth 0)))

(fn `IsDead`
  (`self.K2_DestroyActor` (`self.TestCharacter`))
  (bind _returnvalue (`|CreateWidget` "/Game/Widgets/GameOverWidget.GameOverWidget_C" self))
  (`UserWidget.AddToViewport` _returnvalue 0)
  (set `self.bShowMouseCursor` true))

(fn `SetJumping`
  (set `self.CanJump` true)
  (return))

(fn `UserConstructionScript`)